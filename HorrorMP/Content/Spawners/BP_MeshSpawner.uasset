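; BP_MeshSpawner is an actor that randomizes the meshes shown on its four static mesh components when play begins.
; On BeginPlay, an authority check runs Spawn only on the network authority.
; Spawn makes an independent random pick from ArrayOfMeshes for each component, so meshes can repeat, and assigns it to the existing component without creating new actors.
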(event `self.ReceiveBeginPlay`
  (`/Engine/EditorBlueprintResources/ActorMacros.Switch Has Authority`
    (:`Authority`
      (`self.Spawn`))))

(fn `Spawn`
  (bind _outitem (`KismetArrayLibrary.Array_Random` (`self.ArrayOfMeshes`)))
  (`StaticMeshComponent.SetStaticMesh` (`self.StaticMesh`) _outitem)
  (`StaticMeshComponent.SetStaticMesh` (`self.StaticMesh1`) _outitem)
  (`StaticMeshComponent.SetStaticMesh` (`self.StaticMesh2`) _outitem)
  (`StaticMeshComponent.SetStaticMesh` (`self.StaticMesh3`) _outitem))

(fn `UserConstructionScript`)