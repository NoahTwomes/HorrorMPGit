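; Item spawner that, on authority at BeginPlay, scatters one or several actors of a configurable Class onto surfaces found within its Box area.
; Spawn line-traces on Visibility from a random point in the scaled Box to a set Z height, then spawns at the hit plus an offset, aligned to the surface normal.
; Single mode retries until a hit succeeds, while MultipleItems loops through DoN for ItemAmount attempts, so missed traces yield fewer items.
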(event `self.ReceiveBeginPlay`
  (`/Engine/EditorBlueprintResources/ActorMacros.Switch Has Authority`
    (:`Authority`
      (if (`self.Multiple Items`)
        (bind _counter (`/Engine/EditorBlueprintResources/StandardMacros.Do N` (`self.ItemAmount`) :!label _label)
          (:`Exit`
            (`self.Spawn`)
            (if (not (== _counter (`self.ItemAmount`)))
              (goto _label))))
        (else
          (while (not (`self.Spawned`))
            (`self.Spawn`)))))))

(event `self.ReceiveTick`
  (params (DeltaSeconds :type "Float (single-precision)")))

(fn `Spawn`
  (bind _dividebox (`self.DivideBox`))
  (bind _returnvalue (`KismetMathLibrary.RandomPointInBoundingBox` (`SceneComponent.K2_GetComponentLocation` (`self.Box`)) (`KismetMathLibrary.MakeVector` (/ (.x (`BoxComponent.GetUnscaledBoxExtent` (`self.Box`))) _dividebox) (* (.y (`BoxComponent.GetUnscaledBoxExtent` (`self.Box`))) (`self.Y Value`)) (/ (.z (`BoxComponent.GetUnscaledBoxExtent` (`self.Box`))) _dividebox))))
  (bind (_outhit _returnvalue_2) (`KismetSystemLibrary.LineTraceSingle` :`Start` _returnvalue :`End` (`KismetMathLibrary.MakeVector` (.x _returnvalue) (.y _returnvalue) (`self.Z`)) :`TraceChannel` "TraceTypeQuery1" :`DrawTime` 15.0))
  (if _returnvalue_2
    (bind (_bblockinghit _binitialoverlap _time _distance _location _impactpoint _normal) (`GameplayStatics.BreakHitResult` _outhit))
    (set `self.Spawned` _bblockinghit)
    (set `self.Distance` _distance)
    (`|SpawnActorFromClass` (`self.Class`) (`KismetMathLibrary.MakeTransform` (+ _location (`self.Location`)) (`KismetMathLibrary.MakeRotator` (.roll (`KismetMathLibrary.Conv_VectorToRotator` _normal)) (- (.pitch (`KismetMathLibrary.Conv_VectorToRotator` _normal)) 90.0) (.yaw (`KismetMathLibrary.Conv_VectorToRotator` _normal)))) "Undefined" "MultiplyWithRoot" null null)
    (set `self.Spawned` true)))

(fn `UserConstructionScript`)