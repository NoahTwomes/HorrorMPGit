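; BP_DrawSpawner is a spawner actor that places a single instance of its configured Class at one of three candidate points.
; On BeginPlay it calls Spawn only with authority, so the server decides the placement.
; Spawn picks a random component from Spawn1, Spawn2 and Spawn3, uses its world location, then sets IsSpawned and prints a debug message.
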(event `self.ReceiveBeginPlay`
  (`/Engine/EditorBlueprintResources/ActorMacros.Switch Has Authority`
    (:`Authority`
      (`self.Spawn`))))

(fn `Spawn`
  (`|SpawnActorFromClass` (`self.Class`) (`KismetMathLibrary.MakeTransform` (`SceneComponent.K2_GetComponentLocation` (`KismetArrayLibrary.Array_Random` (`|MakeArray` (`self.Spawn3`) (`self.Spawn2`) (`self.Spawn1`))))) "Undefined" "MultiplyWithRoot" null null)
  (set `self.IsSpawned` true)
  (`KismetSystemLibrary.PrintString` "Spawned"))

(fn `UserConstructionScript`)