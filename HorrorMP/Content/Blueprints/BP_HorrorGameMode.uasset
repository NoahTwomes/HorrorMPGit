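; BP_HorrorGameMode is a horror game mode meant to reveal an exit door once the objective count is met.
; BeginPlay caches the game state and item spawners, then polls objective progress on a looping timer to unhide a random ExitDoors entry and enable its collision.
; Monster spawning and the ExitDoors lookup are disconnected, and the authority switch leads nowhere.
; Tick stores and prints the player count.
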(event `self.ReceiveBeginPlay`
  (bind _asbp_game_state_base (cast `/Game/Blueprints/BP_GameStateBase` (`GameplayStatics.GetGameState`)))
  (set `self.As BP Game State Base` _asbp_game_state_base)
  (`|ExecutionSequence`
    (:`then_0`
      (bind _outactors (`GameplayStatics.GetAllActorsOfClass` "/Game/Spawners/BP_ItemSpawner.BP_ItemSpawner_C"))
      (set `self.ItemSpawnArray` _outactors))
    (:`then_1`
      (`KismetSystemLibrary.K2_SetTimerDelegate` (delegate `AddDoor`) 1.0 true))
    (:`then_2`
      (`/Engine/EditorBlueprintResources/ActorMacros.Switch Has Authority`))
    (:`then_3`
      (`KismetSystemLibrary.Delay` 30.0))))

(event `AddDoor`
  (bind _as_bp_game_state_base (`self.As BP Game State Base`))
  (bind _outitem (`KismetArrayLibrary.Array_Random` (`self.ExitDoors`)))
  (if (>= (`/Game/Blueprints/BP_GameStateBase.ObjectiveAmountCurrent` _as_bp_game_state_base) (`/Game/Blueprints/BP_GameStateBase.ObjectiveAmountTotal` _as_bp_game_state_base))
    (`self.SetActorEnableCollision` _outitem true)
    (`self.SetActorHiddenInGame` _outitem false)))

(event `self.ReceiveTick`
  (params (DeltaSeconds :type "Float (single-precision)"))
  (bind _returnvalue (`self.GetNumPlayers`))
  (bind _output_get (set `self.CurrentPlayers` _returnvalue))
  (`KismetSystemLibrary.PrintString` (`KismetStringLibrary.Conv_IntToString` _output_get)))

(fn `UserConstructionScript`)