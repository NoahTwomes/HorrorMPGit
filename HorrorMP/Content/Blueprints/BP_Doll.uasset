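; BP_Doll is a doll that randomly cries, emitting AI-audible noise at its location with the player pawn as instigator.
; A timer set on BeginPlay rolls a random integer up to Max, triggering the cry on a few low values.
; While an actor overlaps, a second timer lowers Max, raising the odds.
; A cry clears the roll timer without restarting it, then resets Max after a delay.
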(event `self.ReceiveBeginPlay`
  (bind _returnvalue (`KismetSystemLibrary.K2_SetTimerDelegate` (delegate `Noise`) 0.5 (not (`self.IsPlaying`))))
  (set `self.NoiseHandle` _returnvalue))

(event `Noise`
  (bind _returnvalue (`self.K2_GetActorLocation`))
  (switch `int` (`KismetMathLibrary.RandomIntegerInRange` 0 (`self.Max`))
    (:`1`
      _)
    (:`2`
      _)
    (:`3`
      _))
  (`KismetSystemLibrary.K2_ClearAndInvalidateTimerHandle` (`self.NoiseHandle`))
  (set `self.IsPlaying` true)
  (`GameplayStatics.PlaySoundAtLocation` "/Game/Blueprints/angry-baby-cry-36152_Cue.angry-baby-cry-36152_Cue" _returnvalue (struct) 1.0 1.0 0.0 null null null null)
  (`self.MakeNoise` 1.0 (`GameplayStatics.GetPlayerPawn` 0) _returnvalue)
  (`KismetSystemLibrary.Delay` 5.0)
  (set `self.IsPlaying` false)
  (set `self.Max` 1000))

(event `self.ReceiveActorBeginOverlap`
  (params (OtherActor :type "Actor Object Reference"))
  (bind _returnvalue (`KismetSystemLibrary.K2_SetTimerDelegate` (delegate `ReduceMax`) 0.1 true))
  (set `self.MaxTimerHandle` _returnvalue))

(event `ReduceMax`
  (if (> (`self.Max`) 3)
    (set `self.Max` (- (`self.Max`) 1))))

(event `self.ReceiveActorEndOverlap`
  (params (OtherActor :type "Actor Object Reference"))
  (`KismetSystemLibrary.K2_ClearAndInvalidateTimerHandle` (`self.MaxTimerHandle`)))

(event `self.ReceiveTick`
  (params (DeltaSeconds :type "Float (single-precision)")))

(fn `UserConstructionScript`)