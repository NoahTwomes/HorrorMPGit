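; Game state for a horror game that sets the objective total and detects when all players are dead.
; On BeginPlay it caches BP_HorrorGameMode, then starts a looping one-second timer and randomizes the objective total on authority.
; Both steps depend on that cast succeeding, so neither runs on clients, which have no game mode.
; Despite its name, the RestartGame timer event only sets LoseState when DeadPlayers equals the game mode's CurrentPlayers.
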(event `self.ReceiveBeginPlay`
  (bind _asbp_horror_game_mode (cast `/Game/Blueprints/BP_HorrorGameMode` (`GameplayStatics.GetGameMode`)))
  (set `self.As BP Horror Game Mode` _asbp_horror_game_mode)
  (`KismetSystemLibrary.K2_SetTimerDelegate` (delegate `RestartGame`) 1.0 true)
  (`/Engine/EditorBlueprintResources/ActorMacros.Switch Has Authority`
    (:`Authority`
      (set `self.ObjectiveAmountTotal` (`KismetMathLibrary.RandomFloatInRange` 100.0 175.0)))))

(event `RestartGame`
  (if (== (`self.DeadPlayers`) (`/Game/Blueprints/BP_HorrorGameMode.CurrentPlayers` (`self.As BP Horror Game Mode`)))
    (set `self.Lose State` true)))

(fn `UserConstructionScript`)