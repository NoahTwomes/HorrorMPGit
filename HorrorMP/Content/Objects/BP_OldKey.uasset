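; BP_OldKey is an old key object that takes its appearance and name from an item data reference called Primary.
; On BeginPlay, if Primary is valid, it sets the static mesh from the item's mesh and copies the item's name into ItemName.
; A copy of the same logic sits disconnected in the construction script, so the setup runs only at BeginPlay.
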(event `self.ReceiveBeginPlay`
  (bind _primary_ (`self.Primary `)
    (:`then`
      (`StaticMeshComponent.SetStaticMesh` (`self.StaticMesh`) (`/Game/Data/DT_Item.ItemMesh` _primary_))
      (set `self.ItemName` (`/Game/Data/DT_Item.ItemName` _primary_)))
    (:`else`)))

(fn `UserConstructionScript`)