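; BP_Door is a two-panel door that sets up its left and right mesh components from variables.
; On BeginPlay, each panel receives its own static mesh and scale, plus the same fixed half-turn relative rotation.
; The construction script is empty, so this setup applies only at runtime, and the graph has no opening or interaction logic.
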(event `self.ReceiveBeginPlay`
  (bind _doorl (`self.DoorL`))
  (bind _doorr (`self.DoorR`))
  (`StaticMeshComponent.SetStaticMesh` _doorl (`self.DoorLM`))
  (`SceneComponent.SetRelativeScale3D` _doorl (`self.DoorLScale`))
  (`SceneComponent.K2_SetRelativeRotation` _doorl (struct :`Yaw` -179.999998) false false)
  (`StaticMeshComponent.SetStaticMesh` _doorr (`self.DoorRM`))
  (`SceneComponent.K2_SetRelativeRotation` _doorr (struct :`Yaw` -179.999998) false false)
  (`SceneComponent.SetRelativeScale3D` _doorr (`self.DoorRScale`)))

(fn `UserConstructionScript`)