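; BP_ObjectBase is an object actor that takes on a randomly chosen item's identity, likely as a base class given its name.
; Its Spawn function picks a random entry from NewVar, applies that entry's mesh to the static mesh component and stores its name.
; It also replaces the Tags array with that name, so the item can be identified by tag.
; The event graph and construction script are empty.
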(fn `Spawn`
  (bind _data (`self.data`))
  (set `self.data` (`KismetArrayLibrary.Array_Random` (`self.NewVar`)))
  (`StaticMeshComponent.SetStaticMesh` (`self.StaticMesh`) (`/Game/Data/DT_Item.ItemMesh` _data))
  (bind _output_get (set `self.Item Name` (`/Game/Data/DT_Item.ItemName` _data)))
  (set `self.Tags` (`|MakeArray` _output_get)))

(fn `UserConstructionScript`)