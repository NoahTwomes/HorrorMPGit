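; BP_LevelGenerator builds a random room-based level on the server at BeginPlay, starting from BP_LevelRoom1.
; Each step spawns a random room at a random open exit, then after a short delay checks its overlap boxes, destroying and retrying on overlap.
; Accepted rooms add their exits until the room count runs out.
; It then walls leftover exits and spawns BP_Monster at the last room's enemy spawn point.
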(event `Spawn Room`
  ;[1 1 1] SpawnRoom
  (bind _returnvalue (`|SpawnActorFromClass` "/Game/Generation/BP_LevelRoom1.BP_LevelRoom1_C" (`SceneComponent.K2_GetComponentToWorld` (`self.DefaultSceneRoot`)) "AlwaysSpawn" "MultiplyWithRoot" null null))
  (`KismetArrayLibrary.Array_Append` (`self.Exits List`) (`SceneComponent.GetChildrenComponents` (`/Game/Generation/BP_MasterRoom.Exits Folder` _returnvalue) false)))

(event `Spawn Next Room`
  ;[1 1 1] Spawn Nest Room
  (set `self.Selected Exit` (`KismetArrayLibrary.Array_Random` (`self.Exits List`)))
  (bind _returnvalue (`|SpawnActorFromClass` (`KismetArrayLibrary.Array_Random` (`self.Room List`)) (`SceneComponent.K2_GetComponentToWorld` (`self.Selected Exit`)) "AlwaysSpawn" "MultiplyWithRoot" null null))
  (bind _asbp_master_room (cast `/Game/Generation/BP_MasterRoom` _returnvalue))
  (set `self.Latest Room` _asbp_master_room)
  (`KismetSystemLibrary.Delay` 0.1)
  (`self.Check For Overlap`))

(event `self.ReceiveBeginPlay`
  (`/Engine/EditorBlueprintResources/ActorMacros.Switch Has Authority`
    (:`Authority`
      (`self.Spawn Room`)
      (`self.Spawn Next Room`))))

(event `Add overlapping rooms to list`
  (for _array_element (`SceneComponent.GetChildrenComponents` (`/Game/Generation/BP_MasterRoom.OverlapFolder` (`self.Latest Room`)) false)
    (bind _asbox_collision (cast `BoxComponent` _array_element))
    (`KismetArrayLibrary.Array_Append` (`self.Overlapped List`) (`PrimitiveComponent.GetOverlappingComponents` _asbox_collision))))

(event `Check For Overlap`
  (`self.Add overlapping rooms to list`)
  (if (`KismetArrayLibrary.Array_IsNotEmpty` (`self.Overlapped List`))
    (`KismetArrayLibrary.Array_Clear` (`self.Overlapped List`))
    (`self.K2_DestroyActor` (`self.Latest Room`))
    (`self.Spawn Next Room`)
    (else
      (`KismetArrayLibrary.Array_Clear` (`self.Overlapped List`))
      (set `self.Room Amount` (- (`self.Room Amount`) 1))
      (`KismetArrayLibrary.Array_RemoveItem` (`self.Exits List`) (`self.Selected Exit`))
      (`KismetArrayLibrary.Array_Append` (`self.Exits List`) (`SceneComponent.GetChildrenComponents` (`/Game/Generation/BP_MasterRoom.Exits Folder` (`self.Latest Room`)) false))
      (if (> (`self.Room Amount`) 0)
        (`self.Spawn Next Room`)
        (else
          (`self.Close  Holes`)
          (set `self.LevelComplete` true)
          (`|SpawnActorFromClass` "/Game/NPCS/BP_Monster.BP_Monster_C" (`KismetMathLibrary.MakeTransform` (`SceneComponent.K2_GetComponentLocation` (`/Game/Generation/BP_MasterRoom.EnemySpawn` (`self.Latest Room`)))) "AlwaysSpawn" "MultiplyWithRoot" null null))))))

(event `Close  Holes`
  (for _array_element (`self.Exits List`)
    (`|SpawnActorFromClass` "/Game/Generation/BP_ExitWall.BP_ExitWall_C" (`SceneComponent.K2_GetComponentToWorld` _array_element) "AlwaysSpawn" "MultiplyWithRoot" null null)))

(fn `UserConstructionScript`)